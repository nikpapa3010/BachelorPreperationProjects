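; BP_test is a scratch test Blueprint with placeholder logic and no clear gameplay purpose.
; On actor overlap, a valid owner on the other actor triggers TestFunction and an AudioVolume loop of tag lookups, prints and stat queries.
; An invalid owner prints an appended test string, then calls TestFunction, which only holds an empty literal branch.
; BeginPlay and Tick do nothing, and disconnected Sequence nodes remain in the graph.
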(event `self.ReceiveActorBeginOverlap`
  (params (OtherActor :type "Actor Object Reference"))
  (if (`KismetSystemLibrary.IsValid` (`self.GetOwner` OtherActor))
    (bind _outactors (`GameplayStatics.GetAllActorsOfClass` "/Script/Engine.AudioVolume"))
    (`self.testFunction`)
    (if true
      (for _ _outactors
        (`GameplayStatics.GetAllActorsWithTag` "None")
        (`KismetSystemLibrary.PrintString` "Hello")
        (`AutomationBlueprintFunctionLibrary.GetStatCallCount` "None"))
      (else
        (`self.testFunction` :!label _label)))
    (else
      (`KismetSystemLibrary.PrintString` (`KismetStringLibrary.Concat_StrStr` (`self.StringVar`) "test"))
      (goto _label))))

(event `self.ReceiveBeginPlay`
  (if true
    _))

(fn `testFunction`
  (if true
    _))

(fn `UserConstructionScript`)